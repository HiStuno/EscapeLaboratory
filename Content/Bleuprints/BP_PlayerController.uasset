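; Player controller that drives the first-person BP_Body character through Enhanced Input actions for movement, looking and interaction.
; Movement follows the first-person camera's yaw, while look input feeds the character's controller yaw and pitch.
; Interaction fires a short, debug-drawn visibility line trace from the camera and calls OpenDoor on any BP_LabDoor01 it hits.
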(event `EnhancedInput|/Game/EurileneGene/Inputs/Action/IA_Move`
  (params (ActionValue :type "Vector2D Structure") (ElapsedSeconds :type "Float (double-precision)") (TriggeredSeconds :type "Float (double-precision)") (InputAction :type "InputAction Object Reference" :default "/Game/EurileneGene/Inputs/Action/IA_Move.IA_Move"))
  (bind _returnvalue (`GameplayStatics.GetPlayerCharacter` 0))
  ;[0.006671 0.151 0] Controls
  (:`Triggered`
    (bind _asbp_body (cast `/Game/EurileneGene/Core/BP_Body` _returnvalue))
    (bind (_returnvalue_roll _returnvalue_pitch _returnvalue_yaw) (`KismetMathLibrary.BreakRotator` (`SceneComponent.K2_GetComponentRotation` (`/Game/EurileneGene/Core/BP_Body.FirstPersonCamera` _asbp_body))))
    (`Pawn.AddMovementInput` _returnvalue (`KismetMathLibrary.GetForwardVector` (`KismetMathLibrary.MakeRotator` 0.0 0.0 _returnvalue_yaw)) ActionValue_X false)
    (`Pawn.AddMovementInput` _returnvalue (`KismetMathLibrary.GetRightVector` (`KismetMathLibrary.MakeRotator` 0.0 0.0 _returnvalue_yaw)) ActionValue_Y false)))

(event `EnhancedInput|/Game/EurileneGene/Inputs/Action/IA_Interaction`
  (params (ActionValue :type Boolean) (ElapsedSeconds :type "Float (double-precision)") (TriggeredSeconds :type "Float (double-precision)") (InputAction :type "InputAction Object Reference" :default "/Game/EurileneGene/Inputs/Action/IA_Interaction.IA_Interaction"))
  ;[0 0.3281 0] NeuralPsychicInteractionV2.0
  (:`Triggered`
    (bind _asbp_body (cast `/Game/EurileneGene/Core/BP_Body` (`GameplayStatics.GetPlayerCharacter` 0)))
    (bind _firstpersoncamera (`/Game/EurileneGene/Core/BP_Body.FirstPersonCamera` _asbp_body))
    (bind _returnvalue (`SceneComponent.K2_GetComponentLocation` _firstpersoncamera))
    (bind _outhit (`KismetSystemLibrary.LineTraceSingle` :`Start` _returnvalue :`End` (+ _returnvalue (* (`SceneComponent.GetForwardVector` _firstpersoncamera) 200.0)) :`TraceChannel` "TraceTypeQuery1" :`DrawDebugType` "ForDuration"))
    (bind _asbp_lab_door_01 (cast `/Game/ScienceLab/Blueprints/Rooms/Doors/BP_LabDoor01` (`.HitActor` (`GameplayStatics.BreakHitResult` _outhit))))
    (`/Game/ScienceLab/Blueprints/Rooms/Doors/BP_LabDoor01.OpenDoor` _asbp_lab_door_01)))

(event `EnhancedInput|/Game/EurileneGene/Inputs/Action/IA_Look`
  (params (ActionValue :type "Vector2D Structure") (ElapsedSeconds :type "Float (double-precision)") (TriggeredSeconds :type "Float (double-precision)") (InputAction :type "InputAction Object Reference" :default "/Game/EurileneGene/Inputs/Action/IA_Look.IA_Look"))
  (bind _returnvalue (`GameplayStatics.GetPlayerCharacter` 0))
  ;[0.006671 0.151 0] HeadRotation
  (:`Triggered`
    (`Pawn.AddControllerYawInput` _returnvalue ActionValue_X)
    (`Pawn.AddControllerPitchInput` _returnvalue ActionValue_Y)))

(fn `UserConstructionScript`)